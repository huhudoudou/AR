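; Interactive forest scene actor that reacts to touch with animal animations, sounds and rain effects.
; Touching the dog sphere plays a bark animation and sound, while the snail sphere plays a walk animation.
; Three boxes each toggle their own Niagara component and a rain sound, all sharing one RainSound reference.
; Screen touch press and release switch the WPG_Interact canvas between Visible and SelfHitTestInvisible.
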(event OnInputTouchBegin(Sphere_Dog)
  (params (FingerIndex :type ETouchIndex%20Enum :default "Touch1") (TouchedComponent :type Primitive%20Component%20Object%20Reference))
  (Components|Animation|PlayAnimation (Variables|Default|GetDog) "/Game/mx2/Dog/dog2_bark_Anim.dog2_bark_Anim" false)
  (Audio|PlaySound2D "/Game/BP/Audios/Audios_DogBark.Audios_DogBark" 1.0 1.0 0.0 0 0))

(event OnBeginCursorOver(Sphere_Dog)
  (params (TouchedComponent :type Primitive%20Component%20Object%20Reference)))

(event OnEndCursorOver(Sphere_Dog)
  (params (TouchedComponent :type Primitive%20Component%20Object%20Reference)))

(event OnInputTouchBegin(Sphere_Snail)
  (params (FingerIndex :type ETouchIndex%20Enum :default "Touch1") (TouchedComponent :type Primitive%20Component%20Object%20Reference))
  (Components|Animation|PlayAnimation (Variables|Default|GetSnail) "/Game/mx2/Snail/Snails_Anim_Walk.Snails_Anim_Walk" false))

(event OnInputTouchBegin(Box_1)
  (params (FingerIndex :type ETouchIndex%20Enum :default "Touch1") (TouchedComponent :type Primitive%20Component%20Object%20Reference))
  (bind _niagara (Variables|Default|GetNiagara))
  (if (Variables|Default|GetBIsClick1)
    (Rendering|SetVisibility _niagara false false)
    (Variables|Default|SetBIsClick1 false)
    (Audio|Components|Audio|Stop (Variables|Default|GetRainSound))
    (else
      (Rendering|SetVisibility _niagara true false)
      (Variables|Default|SetBIsClick1 true)
      (bind _returnvalue (Audio|SpawnSound2D "/Game/BP/Audios/LightRain_1.LightRain_1" 1.0 1.0 0.0 0))
      (Variables|Default|SetRainSound _returnvalue))))

(event OnInputTouchBegin(Box_2)
  (params (FingerIndex :type ETouchIndex%20Enum :default "Touch1") (TouchedComponent :type Primitive%20Component%20Object%20Reference))
  (bind _niagara1 (Variables|Default|GetNiagara1))
  (if (Variables|Default|GetBIsClick2)
    (Rendering|SetVisibility _niagara1 false false)
    (Variables|Default|SetBIsClick2 false)
    (Audio|Components|Audio|Stop (Variables|Default|GetRainSound))
    (else
      (Rendering|SetVisibility _niagara1 true false)
      (Variables|Default|SetBIsClick2 true)
      (bind _returnvalue (Audio|SpawnSound2D "/Game/BP/Audios/LightRain_1.LightRain_1" 1.0 1.0 0.0 0))
      (Variables|Default|SetRainSound _returnvalue))))

(event OnInputTouchBegin(Box_3)
  (params (FingerIndex :type ETouchIndex%20Enum :default "Touch1") (TouchedComponent :type Primitive%20Component%20Object%20Reference))
  (bind _niagara2 (Variables|Default|GetNiagara2))
  (if (Variables|Default|GetBIsClick3)
    (Rendering|SetVisibility _niagara2 false false)
    (Variables|Default|SetBIsClick3 false)
    (Audio|Components|Audio|Stop (Variables|Default|GetRainSound))
    (else
      (Rendering|SetVisibility _niagara2 true false)
      (Variables|Default|SetBIsClick3 true)
      (bind _returnvalue (Audio|SpawnSound2D "/Game/BP/Audios/LightRain_1.LightRain_1" 1.0 1.0 0.0 0))
      (Variables|Default|SetRainSound _returnvalue))))

(event EventBeginPlay
  (Utilities|FlowControl|Sequence
    (:then_0
      (Input|EnableInput (Game|GetPlayerController 0)))
    (:then_1
      (Variables|Default|SetInitialRotation (Transformation|GetActorRotation))
      (Variables|Default|SetInitialScale (Transformation|GetActorScale3D)))))

(event Collision|EventActorBeginOverlap
  (params (OtherActor :type Actor%20Object%20Reference)))

(event Input|TouchEvents|InputTouch
  (params (Location :type Vector) (FingerIndex :type ETouchIndex%20Enum))
  (:Pressed
    (bind _foundwidgets (Widget|GetAllWidgetsOfClass "/Game/BP/UI/WPG_Interact.WPG_Interact_C" true))
    (Widget|SetVisibility (Variables|/Game/BP/UI/WPG_Interact.WPG_Interact_C|GetCanvasPanel_Interact (Utilities|Array|Get(acopy) _foundwidgets)) "Visible"))
  (:Released
    (bind _foundwidgets_2 (Widget|GetAllWidgetsOfClass "/Game/BP/UI/WPG_Interact.WPG_Interact_C" true))
    (Widget|SetVisibility (Variables|/Game/BP/UI/WPG_Interact.WPG_Interact_C|GetCanvasPanel_Interact (Utilities|Array|Get(acopy) _foundwidgets_2)) "SelfHitTestInvisible")))

(fn ConstructionScript)