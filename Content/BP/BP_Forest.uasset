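; Interactive forest scene actor where touching collision regions triggers sounds, effects, animations and material changes.
; Three boxes toggle shared Niagara rain and sound through separate flags; animal touches play sounds or animations, and the deer sphere briefly deactivates its Niagara effect.
; Door, light and tree touches swap material slots on the forest mesh, with lights and trees reverting after a delay.
; General touch input also changes the WPG_Interact canvas visibility.
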(event OnInputTouchBegin(Sphere_Dog)
  (params (FingerIndex :type ETouchIndex%20Enum :default "Touch1") (TouchedComponent :type Primitive%20Component%20Object%20Reference))
  ;[1 1 1] Animal
  (Components|Animation|PlayAnimation (Variables|Default|GetDog) "/Game/mx2/Dog/dog2_bark_Anim.dog2_bark_Anim" false)
  (Audio|PlaySound2D "/Game/BP/Audios/Audios_DogBark.Audios_DogBark" 1.0 1.0 0.0 0 0))

(event OnInputTouchBegin(Sphere)
  (params (FingerIndex :type ETouchIndex%20Enum :default "Touch1") (TouchedComponent :type Primitive%20Component%20Object%20Reference))
  ;[1 1 1] Deer
  (Audio|PlaySound2D "/Game/BP/Audios/Audios_Deer_2.Audios_Deer_2" 1.0 1.0 0.0 0 0)
  (Components|Activation|SetActive (Variables|Default|GetNS_Deer) false false)
  (Utilities|FlowControl|Delay 4.0)
  (Components|Activation|SetActive (Variables|Default|GetNS_Deer) true false))

(event OnInputTouchBegin(Light_3)
  (params (FingerIndex :type ETouchIndex%20Enum :default "Touch1") (TouchedComponent :type Primitive%20Component%20Object%20Reference))
  ;[1 1 1] Light
  (Rendering|Material|SetMaterial (Variables|Default|GetSM_Forest) 62 "/Game/mx2/Board/MI_Light_Green.MI_Light_Green")
  (Utilities|FlowControl|Delay 3.0)
  (Rendering|Material|SetMaterial (Variables|Default|GetSM_Forest) 62 "/Game/BP/Mesh/Materials/M_Light_Green.M_Light_Green"))

(event OnInputTouchBegin(Light_4)
  (params (FingerIndex :type ETouchIndex%20Enum :default "Touch1") (TouchedComponent :type Primitive%20Component%20Object%20Reference))
  ;[1 1 1] Light
  (Rendering|Material|SetMaterial (Variables|Default|GetSM_Forest) 65 "/Game/mx2/Board/MI_Light_Green.MI_Light_Green")
  (Utilities|FlowControl|Delay 3.0)
  (Rendering|Material|SetMaterial (Variables|Default|GetSM_Forest) 65 "/Game/BP/Mesh/Materials/M_Light_Green.M_Light_Green"))

(event OnInputTouchBegin(Light_5)
  (params (FingerIndex :type ETouchIndex%20Enum :default "Touch1") (TouchedComponent :type Primitive%20Component%20Object%20Reference))
  ;[1 1 1] Light
  (Rendering|Material|SetMaterial (Variables|Default|GetSM_Forest) 66 "/Game/mx2/Board/MI_Light_Pink.MI_Light_Pink")
  (Utilities|FlowControl|Delay 3.0)
  (Rendering|Material|SetMaterial (Variables|Default|GetSM_Forest) 66 "/Game/BP/Mesh/Materials/M_Light_Pink.M_Light_Pink"))

(event OnInputTouchBegin(Tree_1)
  (params (FingerIndex :type ETouchIndex%20Enum :default "Touch1") (TouchedComponent :type Primitive%20Component%20Object%20Reference))
  ;[1 1 1] Tree
  (CallFunction|SetTree "/Game/BP/Mesh/Materials/Master/MI_3.MI_3")
  (Utilities|FlowControl|Delay 3.0)
  (CallFunction|SetTree "/Game/BP/Mesh/Materials/Master/MI_1.MI_1"))

(event OnInputTouchBegin(Tree_2)
  (params (FingerIndex :type ETouchIndex%20Enum :default "Touch1") (TouchedComponent :type Primitive%20Component%20Object%20Reference))
  ;[1 1 1] Tree
  (CallFunction|SetTree "/Game/BP/Mesh/Materials/Master/MI_3.MI_3")
  (Utilities|FlowControl|Delay 3.0)
  (CallFunction|SetTree "/Game/BP/Mesh/Materials/Master/MI_1.MI_1"))

(event OnInputTouchBegin(Tree_3)
  (params (FingerIndex :type ETouchIndex%20Enum :default "Touch1") (TouchedComponent :type Primitive%20Component%20Object%20Reference))
  ;[1 1 1] Tree
  (CallFunction|SetTree "/Game/BP/Mesh/Materials/Master/MI_3.MI_3")
  (Utilities|FlowControl|Delay 3.0)
  (CallFunction|SetTree "/Game/BP/Mesh/Materials/Master/MI_1.MI_1"))

(event OnInputTouchBegin(Door)
  (params (FingerIndex :type ETouchIndex%20Enum :default "Touch1") (TouchedComponent :type Primitive%20Component%20Object%20Reference))
  ;[1 1 1] Door
  (Rendering|Material|SetMaterial (Variables|Default|GetSM_Forest) 16 "/Game/Sword_Fx/Materials/M_Door.M_Door")
  (Audio|PlaySound2D "/Game/BP/Audios/Audios_BG.Audios_BG" 1.0 1.0 0.0 0 0))

(event OnInputTouchBegin(Goat)
  (params (FingerIndex :type ETouchIndex%20Enum :default "Touch1") (TouchedComponent :type Primitive%20Component%20Object%20Reference))
  ;[1 1 1] Animal
  (Audio|PlaySound2D "/Game/BP/Audios/Goat_1.Goat_1" 1.0 1.0 0.0 0 0)
  (Class|SkeletalMeshComponent|SetAnimClass (Variables|Default|GetSkeletalMesh_Goat) "/Game/Cute_Pet/Animations/Goat/BP_Goat_Anim.BP_Goat_Anim_C"))

(event OnInputTouchBegin(Hourse)
  (params (FingerIndex :type ETouchIndex%20Enum :default "Touch1") (TouchedComponent :type Primitive%20Component%20Object%20Reference))
  ;[1 1 1] Animal
  (Audio|PlaySound2D "/Game/BP/Audios/Hourse.Hourse" 1.0 1.0 0.0 0 0)
  (Class|SkeletalMeshComponent|SetAnimClass (Variables|Default|GetSkeletalMesh_Hourse) "/Game/Cute_Pet/Animations/Horse/BP_Horse_Anim.BP_Horse_Anim_C"))

(event OnInputTouchBegin(Rabbit)
  (params (FingerIndex :type ETouchIndex%20Enum :default "Touch1") (TouchedComponent :type Primitive%20Component%20Object%20Reference))
  ;[1 1 1] Animal
  (Audio|PlaySound2D "/Game/BP/Audios/Rabbit.Rabbit" 1.0 1.0 0.0 0 0)
  (Class|SkeletalMeshComponent|SetAnimClass (Variables|Default|GetSkeletalMesh_Rabbit) "/Game/Cute_Pet/Animations/Rabbit/BP_Rabbit_Anim.BP_Rabbit_Anim_C"))

(event OnInputTouchBegin(Alpaca)
  (params (FingerIndex :type ETouchIndex%20Enum :default "Touch1") (TouchedComponent :type Primitive%20Component%20Object%20Reference))
  ;[1 1 1] Animal
  (Audio|PlaySound2D "/Game/BP/Audios/Alpaca.Alpaca" 1.0 1.0 0.0 0 0)
  (Class|SkeletalMeshComponent|SetAnimClass (Variables|Default|GetSkeletalMesh_Alpaca) "/Game/Cute_Pet/Animations/Alpaca/BP_Alpaca_Anim.BP_Alpaca_Anim_C"))

(event OnInputTouchBegin(Light_1)
  (params (FingerIndex :type ETouchIndex%20Enum :default "Touch1") (TouchedComponent :type Primitive%20Component%20Object%20Reference))
  ;[1 1 1] Light
  (CallFunction|SetLight 68 70 "/Game/mx2/Board/MI_Light_Green.MI_Light_Green" "/Game/mx2/Board/MI_Light_Pink.MI_Light_Pink")
  (Utilities|FlowControl|Delay 3.0)
  (CallFunction|SetLight 68 70 "/Game/BP/Mesh/Materials/M_Light_Green.M_Light_Green" "/Game/BP/Mesh/Materials/M_Light_Pink.M_Light_Pink"))

(event OnInputTouchBegin(Sphere_Snail)
  (params (FingerIndex :type ETouchIndex%20Enum :default "Touch1") (TouchedComponent :type Primitive%20Component%20Object%20Reference))
  ;[1 1 1] Animal
  (Components|Animation|PlayAnimation (Variables|Default|GetSnail) "/Game/mx2/Snail/Snails_Anim_Walk.Snails_Anim_Walk" false))

(event OnInputTouchBegin(Box_1)
  (params (FingerIndex :type ETouchIndex%20Enum :default "Touch1") (TouchedComponent :type Primitive%20Component%20Object%20Reference))
  (bind _niagara_rain (Variables|Default|GetNiagara_Rain))
  ;[1 1 1] Comment
  (if (Variables|Default|GetBIsClick1)
    (Rendering|SetVisibility _niagara_rain false false)
    (Variables|Default|SetBIsClick1 false)
    (Audio|Components|Audio|Stop (Variables|Default|GetRainSound))
    (else
      (Rendering|SetVisibility _niagara_rain true false)
      (Variables|Default|SetBIsClick1 true)
      (bind _returnvalue (Audio|SpawnSound2D "/Game/BP/Audios/LightRain_1.LightRain_1" 1.0 1.0 0.0 0))
      (Variables|Default|SetRainSound _returnvalue))))

(event OnInputTouchBegin(Box_2)
  (params (FingerIndex :type ETouchIndex%20Enum :default "Touch1") (TouchedComponent :type Primitive%20Component%20Object%20Reference))
  (bind _niagara_rain (Variables|Default|GetNiagara_Rain))
  ;[1 1 1] Comment
  (if (Variables|Default|GetBIsClick2)
    (Rendering|SetVisibility _niagara_rain false false)
    (Variables|Default|SetBIsClick2 false)
    (Audio|Components|Audio|Stop (Variables|Default|GetRainSound))
    (else
      (Rendering|SetVisibility _niagara_rain true false)
      (Variables|Default|SetBIsClick2 true)
      (bind _returnvalue (Audio|SpawnSound2D "/Game/BP/Audios/LightRain_1.LightRain_1" 1.0 1.0 0.0 0))
      (Variables|Default|SetRainSound _returnvalue))))

(event OnInputTouchBegin(Box_3)
  (params (FingerIndex :type ETouchIndex%20Enum :default "Touch1") (TouchedComponent :type Primitive%20Component%20Object%20Reference))
  (bind _niagara_rain (Variables|Default|GetNiagara_Rain))
  ;[1 1 1] Comment
  (if (Variables|Default|GetBIsClick3)
    (Rendering|SetVisibility _niagara_rain false false)
    (Variables|Default|SetBIsClick3 false)
    (Audio|Components|Audio|Stop (Variables|Default|GetRainSound))
    (else
      (Rendering|SetVisibility _niagara_rain true false)
      (Variables|Default|SetBIsClick3 true)
      (bind _returnvalue (Audio|SpawnSound2D "/Game/BP/Audios/LightRain_1.LightRain_1" 1.0 1.0 0.0 0))
      (Variables|Default|SetRainSound _returnvalue))))

(event OnInputTouchBegin(Light_2)
  (params (FingerIndex :type ETouchIndex%20Enum :default "Touch1") (TouchedComponent :type Primitive%20Component%20Object%20Reference))
  ;[1 1 1] Light
  (CallFunction|SetLight 75 77 "/Game/mx2/Board/MI_Light_Green.MI_Light_Green" "/Game/mx2/Board/MI_Light_Pink.MI_Light_Pink")
  (Utilities|FlowControl|Delay 3.0)
  (CallFunction|SetLight 75 77 "/Game/BP/Mesh/Materials/M_Light_Green.M_Light_Green" "/Game/BP/Mesh/Materials/M_Light_Pink.M_Light_Pink"))

(event EventBeginPlay
  (Utilities|FlowControl|Sequence
    (:then_0
      (Input|EnableInput (Game|GetPlayerController 0)))
    (:then_1
      (Variables|Default|SetInitialRotation (Transformation|GetActorRotation))
      (Variables|Default|SetInitialScale (Transformation|GetActorScale3D)))))

(event Collision|EventActorBeginOverlap
  (params (OtherActor :type Actor%20Object%20Reference)))

(event Input|TouchEvents|InputTouch
  (params (Location :type Vector) (FingerIndex :type ETouchIndex%20Enum))
  (:Pressed
    (bind _foundwidgets (Widget|GetAllWidgetsOfClass "/Game/BP/UI/WPG_Interact.WPG_Interact_C" true))
    (Widget|SetVisibility (Variables|/Game/BP/UI/WPG_Interact.WPG_Interact_C|GetCanvasPanel_Interact (Utilities|Array|Get(acopy) _foundwidgets)) "Visible"))
  (:Released
    (bind _foundwidgets_2 (Widget|GetAllWidgetsOfClass "/Game/BP/UI/WPG_Interact.WPG_Interact_C" true))
    (Widget|SetVisibility (Variables|/Game/BP/UI/WPG_Interact.WPG_Interact_C|GetCanvasPanel_Interact (Utilities|Array|Get(acopy) _foundwidgets_2)) "SelfHitTestInvisible")))

(fn ConstructionScript)

(fn SetLight
  (params (Index1 :type Integer) (Index2 :type Integer) (Material :type Material%20Interface%20Object%20Reference) (Material1 :type Material%20Interface%20Object%20Reference))
  (bind _sm_forest (Variables|Default|GetSM_Forest))
  (Rendering|Material|SetMaterial _sm_forest Index1 Material)
  (Rendering|Material|SetMaterial _sm_forest Index2 Material1))

(fn SetTree
  (params (Material :type Material%20Interface%20Object%20Reference))
  (for _array_element (Variables|Default|GetIndex)
    (Rendering|Material|SetMaterial (Variables|Default|GetSM_Forest) _array_element Material)))